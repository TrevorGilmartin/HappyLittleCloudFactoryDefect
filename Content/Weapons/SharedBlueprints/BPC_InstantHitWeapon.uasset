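; Base instant-hit weapon Blueprint that, on Fire, checks and decrements ammo, shows muzzle flash and runs hitscan traces toward the crosshair.
; Multiple debug-drawn traces scatter randomly within a spread cone, but results are stored only while no hit has registered.
; If any trace hits, stored results receive point damage and impact effects from the ammo's settings.
; Fire and no-ammo sound functions do nothing, with fire-sound logic left disconnected.
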(event `OnFire`
  (params (CrossHairWorldSpace :type "Vector Structure"))
  ;[1 1 1] On Fire - Workflow when weapon is fired by a character
  (bind _canfire (`self.CanWeaponFire`))
  (if _canfire
    (`self.DecrementAmmo`)
    (`self.PlayMuzzelFlash`)
    (`self.PlayFireSound`)
    (bind _hitoccured_ (`self.DetermineHitObjects` CrossHairWorldSpace))
    (if _hitoccured_
      (`self.ApplyDamageToHitActors`)
      (`self.PlayImpactEffects`))
    (else
      (`self.PlayNoAmmoSound`))))

(fn `ApplyDamageToHitActors`
  (bind _returnvalue (`self.GetInstigatorController`))
  (for _index (range (`KismetArrayLibrary.Array_Length` (`self.HitResult`)))
    (bind _item (`KismetArrayLibrary.Array_Get` (`self.HitResult`) _index))
    (bind (_bblockinghit _binitialoverlap _time _location _impactpoint _normal _impactnormal _physmat _hitactor) (`GameplayStatics.BreakHitResult` _item))
    (`GameplayStatics.ApplyPointDamage` _hitactor (`/Game/Weapons/SharedBlueprints/BP_AmmoBase.BaseDamage` (`self.BP_AmmoBase`)) (`KismetMathLibrary.Conv_RotatorToVector` (`KismetMathLibrary.FindLookAtRotation` _location (`self.K2_GetActorLocation` (`Controller.K2_GetPawn` _returnvalue)))) _item _returnvalue self)))

(fn `CanWeaponFire`
  (returns (CanFire :type Boolean))
  (if (> (`self.Ammo`) 0.0)
    (set `self.CanFire?` true)
    (else
      (set `self.CanFire?` false)))
  (return (`self.CanFire?`)))

(fn `DecrementAmmo`
  (set `self.Ammo` (`KismetMathLibrary.FClamp` (- (`self.Ammo`) 1.0) 0.0 (`self.MaxAmmo`))))

(fn `DetermineHitObjects`
  (params (CrosshairWorldSpace :type "Vector Structure"))
  (returns (`HitOccured?` :type Boolean))
  (locals (`ObjectHit?` :type Boolean))
  (bind _returnvalue (`SceneComponent.GetSocketLocation` (`self.Mesh`) (`self.MuzzelSocket`)))
  (`KismetArrayLibrary.Array_Clear` (`self.HitResult`))
  (for _ (range (`self.TracesUsed`))
    (bind (_outhit _returnvalue_2) (`KismetSystemLibrary.LineTraceSingle` :`Start` _returnvalue :`End` (+ _returnvalue (`KismetMathLibrary.GreaterGreater_VectorRotator` (* (`KismetMathLibrary.RandomUnitVectorInCone` (-1.0 0.0 0.0) (`KismetMathLibrary.DegreesToRadians` (`self.Spread`))) (`self.Range`)) (`KismetMathLibrary.FindLookAtRotation` _returnvalue CrosshairWorldSpace))) :`TraceChannel` "TraceTypeQuery1" :`DrawDebugType` "ForDuration"))
    (bind _output_get (set `local.ObjectHit?` (or _returnvalue_2 (`local.ObjectHit?`))))
    (if (not _output_get)
      (`KismetArrayLibrary.Array_Append` (`self.HitResult`) (`|MakeArray` _outhit))))
  (return (`local.ObjectHit?`)))

(fn `PlayFireSound`)

(fn `PlayImpactEffects`
  (bind _bp_ammobase (`self.BP_AmmoBase`))
  (for _index (range (`KismetArrayLibrary.Array_Length` (`self.HitResult`)))
    (bind (_bblockinghit _binitialoverlap _time _location) (`GameplayStatics.BreakHitResult` (`KismetArrayLibrary.Array_Get` (`self.HitResult`) _index)))
    (`GameplayStatics.SpawnEmitterAtLocation` (`/Game/Weapons/SharedBlueprints/BP_AmmoBase.ImpactParticleSystem` _bp_ammobase) _location)
    (`GameplayStatics.SpawnSoundAtLocation` (`/Game/Weapons/SharedBlueprints/BP_AmmoBase.ImpactSound` _bp_ammobase) _location)))

(fn `PlayMuzzelFlash`
  (bind _mesh (`self.Mesh`))
  (bind _muzzelsocket (`self.MuzzelSocket`))
  (`GameplayStatics.SpawnEmitterAttached` (`self.MuzzelFlash`) _mesh _muzzelsocket (`SceneComponent.GetSocketLocation` _mesh _muzzelsocket) (`SceneComponent.GetSocketRotation` _mesh _muzzelsocket)))

(fn `PlayNoAmmoSound`)

(fn `UserConstructionScript`
  (`parent.UserConstructionScript`))